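; Base AI character that patrols, chases sensed targets and searches when it loses them, with debug prints throughout.
; AIPerception updates toggle CanSeePlayer, triggering either a chase or a search from the last stimulus location.
; The search visits a few random navmesh points within a growing radius, then resumes the looping random patrol around itself.
; All movement uses AIMoveTo in the event graph, and the action on reaching the player is a placeholder print.
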(event `self.ReceiveBeginPlay`
  (`self.ReturnToPatrol`))

(event `self.AIPerception.OnTargetPerceptionUpdated`
  (params (Actor :type "Actor Object Reference") (Stimulus :type "AIStimulus Structure"))
  ;[1 1 1] AIPerception target updated - Set or Unset CanSeePlayer, start go to player or search for player if we can see player or not
  (if Stimulus_bSuccessfullySensed
    (`KismetSystemLibrary.PrintString` "See character")
    (set `self.CanSeePlayer?` true)
    (`self.GoToPlayer` Actor)
    (else
      (`KismetSystemLibrary.PrintString` "Cannot see character")
      (set `self.CanSeePlayer?` false)
      (`self.SearchForPlayer` Stimulus_StimulusLocation))))

(event `GoToPlayer`
  (params (Player :type "Actor Object Reference"))
  ;[1 1 1] GoToPlayer - if near player do something (attack for exemple)
  (`KismetSystemLibrary.PrintString` "GoToPlayer" true true (struct :`R` 1.0 :`G` 0.805564 :`A` 1.0))
  (`MovementComponent.StopMovementImmediately` (`self.CharacterMovement`))
  (`|AIMoveTo` self (0.0 0.0 0.0) Player 10.0 true
    (:`OnSuccess`
      _)
    (:`OnFail`
      _))
  (if (`self.CanSeePlayer?`)
    (`KismetSystemLibrary.PrintString` "I am near player do something" true true (struct :`R` 1.0 :`G` 0.805564 :`A` 1.0))))

(event `SearchForPlayer`
  (params (LastSeenPlayerLocation :type "Vector Structure"))
  ;[1 1 1] Search for player - Go to last seen player location if can see player follow him, if not, increase radius range from the location we have last time seen him and look for him arround this radius, repeat X times, if see player follows him, if not after X iteration goes to patrol
  (`KismetSystemLibrary.PrintString` "SearchForPlayer" true true (struct :`R` 1.0 :`G` 0.805564 :`A` 1.0))
  (set `self.LocToSearchPlayer` LastSeenPlayerLocation)
  (`MovementComponent.StopMovementImmediately` (`self.CharacterMovement`))
  (`|AIMoveTo` self (`self.LocToSearchPlayer`) null 10.0 true
    (:`OnSuccess`
      _)
    (:`OnFail`
      _))
  (`KismetSystemLibrary.Delay` (`KismetMathLibrary.RandomFloatInRange` 1.0 3.0))
  (if (`self.CanSeePlayer?`)
    (`self.GoToPlayer` (`GameplayStatics.GetPlayerCharacter` 0))
    (else
      (if (< (`self.i`) 3) :!label _label
        (`/Engine/EditorBlueprintResources/StandardMacros.IncrementInt` (`self.i`)
          (:`  `
            (`KismetSystemLibrary.PrintString` (`KismetStringLibrary.Concat_StrStr` "Search more player : " (`KismetStringLibrary.Conv_IntToString` (`self.i`))) true true (struct :`R` 1.0 :`G` 0.805564 :`A` 1.0))
            (bind _randomlocation (`NavigationSystemV1.K2_GetRandomLocationInNavigableRadius` (`self.LocToSearchPlayer`) (`self.RadiusToSearchPlayer`) null null))
            (bind _output_get (set `self.LocToSearchPlayer` _randomlocation))
            (set `self.RadiusToSearchPlayer` (* (`self.RadiusToSearchPlayer`) 1.5))
            (`|AIMoveTo` self _output_get null
              (:`OnSuccess`
                _)
              (:`OnFail`
                _))
            (`KismetSystemLibrary.Delay` (`KismetMathLibrary.RandomFloatInRange` 1.0 3.0))
            (goto _label)))
        (else
          (set `self.i` 0)
          (set `self.RadiusToSearchPlayer` 500.0)
          (`self.ReturnToPatrol`))))))

(event `ReturnToPatrol`
  ;[1 1 1] Patrol - Get random  point arround this Actor and go there wait X seconds after and then relaunch this function
  (`KismetSystemLibrary.PrintString` "Lost player going to patrol" true true (struct :`R` 1.0 :`G` 0.805564 :`A` 1.0) :!label _label_2)
  (`MovementComponent.StopMovementImmediately` (`self.CharacterMovement`))
  (bind _randomlocation (`NavigationSystemV1.K2_GetRandomLocationInNavigableRadius` (`self.K2_GetActorLocation`) 3000.0 null null))
  (`|AIMoveTo` self _randomlocation null
    (:`OnSuccess`
      _)
    (:`OnFail`
      _))
  (`KismetSystemLibrary.Delay` 5.0)
  (goto _label_2))

(fn `UserConstructionScript`)