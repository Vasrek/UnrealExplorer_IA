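; Base AI pawn Blueprint that relays AI Perception results to its controller's Blackboard for a behavior tree to use in chasing or searching for the player.
; A successful sense sets CanSeePlayer? and clears HasSeenPlayer?.
; A lost sense flips both flags and stores the stimulus location as LastSeenPlayerLocation.
; The handler never checks which actor is sensed and prints debug messages on each update.
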(event `self.AIPerception.OnTargetPerceptionUpdated`
  (params (Actor :type "Actor Object Reference") (Stimulus :type "AIStimulus Structure"))
  (bind _returnvalue (`AIBlueprintHelperLibrary.GetBlackboard` (`AIBlueprintHelperLibrary.GetAIController` self)))
  ;[1 1 1] AIPerception target updated - Set or Unset CanSeePlayer, start go to player or search for player if we can see player or not
  (if Stimulus_bSuccessfullySensed
    (`KismetSystemLibrary.PrintString` "See character")
    (`BlackboardComponent.SetValueAsBool` _returnvalue "CanSeePlayer?" true)
    (`BlackboardComponent.SetValueAsBool` _returnvalue "HasSeenPlayer?" false)
    (else
      (`KismetSystemLibrary.PrintString` "Cannot see character")
      (`BlackboardComponent.SetValueAsBool` _returnvalue "CanSeePlayer?" false)
      (`BlackboardComponent.SetValueAsBool` _returnvalue "HasSeenPlayer?" true)
      (`BlackboardComponent.SetValueAsVector` _returnvalue "LastSeenPlayerLocation" Stimulus_StimulusLocation))))

(fn `UserConstructionScript`)